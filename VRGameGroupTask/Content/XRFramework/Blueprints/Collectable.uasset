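; Collectable is an XR actor that the player picks up by grabbing, then bursts and disappears.
; BeginPlay assigns the collectable mesh and deactivates the Explode effect.
; Any of its five grab components runs one shared sequence: play a 2D shimmer sound, wait, hide the mesh and activate Explode, then destroy the actor after another delay.
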(event OnGrabbed(BP_GrabComponent)
  (Audio|PlaySound2D "/Game/Music/SFX_ANIME_Metallic_Shimmer_001.SFX_ANIME_Metallic_Shimmer_001" 1.0 1.0 0.0 0 0)
  (Utilities|FlowControl|Delay 1.0)
  (Rendering|SetVisibility (Variables|Default|GetStaticMesh) false false)
  (Components|Activation|Activate (Variables|Default|GetExplode) true)
  (Utilities|FlowControl|Delay 1.0)
  (Actor|DestroyActor))

(event OnGrabbed(BP_GrabComponent1)
  (Audio|PlaySound2D "/Game/Music/SFX_ANIME_Metallic_Shimmer_001.SFX_ANIME_Metallic_Shimmer_001" 1.0 1.0 0.0 0 0)
  (Utilities|FlowControl|Delay 1.0)
  (Rendering|SetVisibility (Variables|Default|GetStaticMesh) false false)
  (Components|Activation|Activate (Variables|Default|GetExplode) true)
  (Utilities|FlowControl|Delay 1.0)
  (Actor|DestroyActor))

(event OnGrabbed(BP_GrabComponent2)
  (Audio|PlaySound2D "/Game/Music/SFX_ANIME_Metallic_Shimmer_001.SFX_ANIME_Metallic_Shimmer_001" 1.0 1.0 0.0 0 0)
  (Utilities|FlowControl|Delay 1.0)
  (Rendering|SetVisibility (Variables|Default|GetStaticMesh) false false)
  (Components|Activation|Activate (Variables|Default|GetExplode) true)
  (Utilities|FlowControl|Delay 1.0)
  (Actor|DestroyActor))

(event OnGrabbed(BP_GrabComponent3)
  (Audio|PlaySound2D "/Game/Music/SFX_ANIME_Metallic_Shimmer_001.SFX_ANIME_Metallic_Shimmer_001" 1.0 1.0 0.0 0 0)
  (Utilities|FlowControl|Delay 1.0)
  (Rendering|SetVisibility (Variables|Default|GetStaticMesh) false false)
  (Components|Activation|Activate (Variables|Default|GetExplode) true)
  (Utilities|FlowControl|Delay 1.0)
  (Actor|DestroyActor))

(event OnGrabbed(BP_GrabComponent4)
  (Audio|PlaySound2D "/Game/Music/SFX_ANIME_Metallic_Shimmer_001.SFX_ANIME_Metallic_Shimmer_001" 1.0 1.0 0.0 0 0)
  (Utilities|FlowControl|Delay 1.0)
  (Rendering|SetVisibility (Variables|Default|GetStaticMesh) false false)
  (Components|Activation|Activate (Variables|Default|GetExplode) true)
  (Utilities|FlowControl|Delay 1.0)
  (Actor|DestroyActor))

(event EventBeginPlay
  (Components|StaticMesh|SetStaticMesh (Variables|Default|GetStaticMesh) (Variables|Mesh|GetCollectableMesh))
  (Components|Activation|Deactivate (Variables|Default|GetExplode)))

(fn ConstructionScript)