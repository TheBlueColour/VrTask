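; XR game mode that manages pawn spawning, target score popups and score-gated doors.
; SpawnPlayer spawns a BP_XRPawn at a fixed location after a delay and has the first player controller possess it.
; BeginPlay makes a one-time delayed check of Points against a threshold, destroying two indexed door and target pairs behind done flags.
; Score events briefly set the TargetPoints text, without changing Points.
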(event Custom|SpawnPlayer
  (Utilities|FlowControl|Delay 2.0)
  (bind _returnvalue (Game|SpawnActorfromClass "/Game/XRFramework/Blueprints/BP_XRPawn.BP_XRPawn_C" (Math|Transform|MakeTransform "1965.430902,5955.646074,247.977596" "0, 0, 0" "1.000000,1.000000,1.000000") "Undefined" "MultiplyWithRoot" 0 0))
  (Pawn|Possess (Game|GetPlayerController 0) _returnvalue))

(event Custom|TenPoints
  (Variables|Default|SetTargetPoints "10")
  (Utilities|FlowControl|Delay 0.5)
  (Variables|Default|SetTargetPoints ""))

(event Custom|TwentyPoints
  (Variables|Default|SetTargetPoints "20")
  (Utilities|FlowControl|Delay 0.5)
  (Variables|Default|SetTargetPoints ""))

(event Custom|ThirtyPoints
  (Variables|Default|SetTargetPoints "30")
  (Utilities|FlowControl|Delay 0.5)
  (Variables|Default|SetTargetPoints ""))

(event EventBeginPlay
  (Utilities|FlowControl|Delay 2.0)
  (Utilities|FlowControl|Sequence
    (:then_0
      (if (not (Variables|Default|GetDone1))
        (Math|Integer|CompareInt (Variables|Default|GetPoints) 100
          (:>
            _)
          (:==
            _))
        (bind _outactors (Actor|GetAllActorsOfClass "/Game/XRFramework/Blueprints/BP_Door.BP_Door_C"))
        (Actor|DestroyActor (Utilities|Array|Get(acopy) _outactors))
        (bind _outactors_2 (Actor|GetAllActorsOfClass "/Game/XRFramework/Blueprints/Target.Target_C"))
        (Actor|DestroyActor (Utilities|Array|Get(acopy) _outactors_2))
        (Variables|Default|SetDone1 true)))
    (:then_1
      (if (not (Variables|Default|GetDone2))
        (Math|Integer|CompareInt (Variables|Default|GetPoints) 100
          (:>
            _)
          (:==
            _))
        (bind _outactors_3 (Actor|GetAllActorsOfClass "/Game/XRFramework/Blueprints/BP_Door.BP_Door_C"))
        (Actor|DestroyActor (Utilities|Array|Get(acopy) _outactors_3 1))
        (bind _outactors_4 (Actor|GetAllActorsOfClass "/Game/XRFramework/Blueprints/Target.Target_C"))
        (Actor|DestroyActor (Utilities|Array|Get(acopy) _outactors_4 1))
        (Variables|Default|SetDone2 true)))))

(fn ConstructionScript)