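; Scoring target actor for the XR game that awards points when a BP_Projectile hits one of its zones.
; Nine box components each handle their own begin-overlap event, worth ten, twenty or thirty points by zone.
; Each handler adds to Points on BP_XRGameMode and calls the matching tier event there.
; The same logic is duplicated per box, with no state kept on the target itself.
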(event OnComponentBeginOverlap(Box)
  (params (OverlappedComponent :type Primitive%20Component%20Object%20Reference) (OtherActor :type Actor%20Object%20Reference) (OtherComp :type Primitive%20Component%20Object%20Reference) (OtherBodyIndex :type Integer) (bFromSweep :type Boolean) (SweepResult :type Hit%20Result%20Structure%20%28by%20ref%29))
  (Utilities|Casting|CastToBP_Projectile OtherActor)
  (bind _asbp_xrgame_mode (Utilities|Casting|CastToBP_XRGameMode (Game|GetGameMode)))
  (Variables|/Game/XRFramework/Blueprints/BP_XRGameMode.BP_XRGameMode_C|SetPoints _asbp_xrgame_mode (+ (Variables|/Game/XRFramework/Blueprints/BP_XRGameMode.BP_XRGameMode_C|GetPoints _asbp_xrgame_mode) 10))
  (Default|TenPoints _asbp_xrgame_mode))

(event OnComponentBeginOverlap(Box1)
  (params (OverlappedComponent :type Primitive%20Component%20Object%20Reference) (OtherActor :type Actor%20Object%20Reference) (OtherComp :type Primitive%20Component%20Object%20Reference) (OtherBodyIndex :type Integer) (bFromSweep :type Boolean) (SweepResult :type Hit%20Result%20Structure%20%28by%20ref%29))
  (Utilities|Casting|CastToBP_Projectile OtherActor)
  (bind _asbp_xrgame_mode (Utilities|Casting|CastToBP_XRGameMode (Game|GetGameMode)))
  (Variables|/Game/XRFramework/Blueprints/BP_XRGameMode.BP_XRGameMode_C|SetPoints _asbp_xrgame_mode (+ (Variables|/Game/XRFramework/Blueprints/BP_XRGameMode.BP_XRGameMode_C|GetPoints _asbp_xrgame_mode) 10))
  (Default|TenPoints _asbp_xrgame_mode))

(event OnComponentBeginOverlap(Box5)
  (params (OverlappedComponent :type Primitive%20Component%20Object%20Reference) (OtherActor :type Actor%20Object%20Reference) (OtherComp :type Primitive%20Component%20Object%20Reference) (OtherBodyIndex :type Integer) (bFromSweep :type Boolean) (SweepResult :type Hit%20Result%20Structure%20%28by%20ref%29))
  (Utilities|Casting|CastToBP_Projectile OtherActor)
  (bind _asbp_xrgame_mode (Utilities|Casting|CastToBP_XRGameMode (Game|GetGameMode)))
  (Variables|/Game/XRFramework/Blueprints/BP_XRGameMode.BP_XRGameMode_C|SetPoints _asbp_xrgame_mode (+ (Variables|/Game/XRFramework/Blueprints/BP_XRGameMode.BP_XRGameMode_C|GetPoints _asbp_xrgame_mode) 10))
  (Default|TenPoints _asbp_xrgame_mode))

(event OnComponentBeginOverlap(Box6)
  (params (OverlappedComponent :type Primitive%20Component%20Object%20Reference) (OtherActor :type Actor%20Object%20Reference) (OtherComp :type Primitive%20Component%20Object%20Reference) (OtherBodyIndex :type Integer) (bFromSweep :type Boolean) (SweepResult :type Hit%20Result%20Structure%20%28by%20ref%29))
  (Utilities|Casting|CastToBP_Projectile OtherActor)
  (bind _asbp_xrgame_mode (Utilities|Casting|CastToBP_XRGameMode (Game|GetGameMode)))
  (Variables|/Game/XRFramework/Blueprints/BP_XRGameMode.BP_XRGameMode_C|SetPoints _asbp_xrgame_mode (+ (Variables|/Game/XRFramework/Blueprints/BP_XRGameMode.BP_XRGameMode_C|GetPoints _asbp_xrgame_mode) 10))
  (Default|TenPoints _asbp_xrgame_mode))

(event OnComponentBeginOverlap(Box7)
  (params (OverlappedComponent :type Primitive%20Component%20Object%20Reference) (OtherActor :type Actor%20Object%20Reference) (OtherComp :type Primitive%20Component%20Object%20Reference) (OtherBodyIndex :type Integer) (bFromSweep :type Boolean) (SweepResult :type Hit%20Result%20Structure%20%28by%20ref%29))
  (Utilities|Casting|CastToBP_Projectile OtherActor)
  (bind _asbp_xrgame_mode (Utilities|Casting|CastToBP_XRGameMode (Game|GetGameMode)))
  (Variables|/Game/XRFramework/Blueprints/BP_XRGameMode.BP_XRGameMode_C|SetPoints _asbp_xrgame_mode (+ (Variables|/Game/XRFramework/Blueprints/BP_XRGameMode.BP_XRGameMode_C|GetPoints _asbp_xrgame_mode) 10))
  (Default|TenPoints _asbp_xrgame_mode))

(event OnComponentBeginOverlap(Box8)
  (params (OverlappedComponent :type Primitive%20Component%20Object%20Reference) (OtherActor :type Actor%20Object%20Reference) (OtherComp :type Primitive%20Component%20Object%20Reference) (OtherBodyIndex :type Integer) (bFromSweep :type Boolean) (SweepResult :type Hit%20Result%20Structure%20%28by%20ref%29))
  (Utilities|Casting|CastToBP_Projectile OtherActor)
  (bind _asbp_xrgame_mode (Utilities|Casting|CastToBP_XRGameMode (Game|GetGameMode)))
  (Variables|/Game/XRFramework/Blueprints/BP_XRGameMode.BP_XRGameMode_C|SetPoints _asbp_xrgame_mode (+ (Variables|/Game/XRFramework/Blueprints/BP_XRGameMode.BP_XRGameMode_C|GetPoints _asbp_xrgame_mode) 30))
  (Default|ThirtyPoints _asbp_xrgame_mode))

(event OnComponentBeginOverlap(Box2)
  (params (OverlappedComponent :type Primitive%20Component%20Object%20Reference) (OtherActor :type Actor%20Object%20Reference) (OtherComp :type Primitive%20Component%20Object%20Reference) (OtherBodyIndex :type Integer) (bFromSweep :type Boolean) (SweepResult :type Hit%20Result%20Structure%20%28by%20ref%29))
  (Utilities|Casting|CastToBP_Projectile OtherActor)
  (bind _asbp_xrgame_mode (Utilities|Casting|CastToBP_XRGameMode (Game|GetGameMode)))
  (Variables|/Game/XRFramework/Blueprints/BP_XRGameMode.BP_XRGameMode_C|SetPoints _asbp_xrgame_mode (+ (Variables|/Game/XRFramework/Blueprints/BP_XRGameMode.BP_XRGameMode_C|GetPoints _asbp_xrgame_mode) 10))
  (Default|TenPoints _asbp_xrgame_mode))

(event OnComponentBeginOverlap(Box3)
  (params (OverlappedComponent :type Primitive%20Component%20Object%20Reference) (OtherActor :type Actor%20Object%20Reference) (OtherComp :type Primitive%20Component%20Object%20Reference) (OtherBodyIndex :type Integer) (bFromSweep :type Boolean) (SweepResult :type Hit%20Result%20Structure%20%28by%20ref%29))
  (Utilities|Casting|CastToBP_Projectile OtherActor)
  (bind _asbp_xrgame_mode (Utilities|Casting|CastToBP_XRGameMode (Game|GetGameMode)))
  (Variables|/Game/XRFramework/Blueprints/BP_XRGameMode.BP_XRGameMode_C|SetPoints _asbp_xrgame_mode (+ (Variables|/Game/XRFramework/Blueprints/BP_XRGameMode.BP_XRGameMode_C|GetPoints _asbp_xrgame_mode) 10))
  (Default|TenPoints _asbp_xrgame_mode))

(event OnComponentBeginOverlap(Box4)
  (params (OverlappedComponent :type Primitive%20Component%20Object%20Reference) (OtherActor :type Actor%20Object%20Reference) (OtherComp :type Primitive%20Component%20Object%20Reference) (OtherBodyIndex :type Integer) (bFromSweep :type Boolean) (SweepResult :type Hit%20Result%20Structure%20%28by%20ref%29))
  (Utilities|Casting|CastToBP_Projectile OtherActor)
  (bind _asbp_xrgame_mode (Utilities|Casting|CastToBP_XRGameMode (Game|GetGameMode)))
  (Variables|/Game/XRFramework/Blueprints/BP_XRGameMode.BP_XRGameMode_C|SetPoints _asbp_xrgame_mode (+ (Variables|/Game/XRFramework/Blueprints/BP_XRGameMode.BP_XRGameMode_C|GetPoints _asbp_xrgame_mode) 20))
  (Default|TwentyPoints _asbp_xrgame_mode))

(event EventBeginPlay)

(event Collision|EventActorBeginOverlap
  (params (OtherActor :type Actor%20Object%20Reference)))

(event EventTick
  (params (DeltaSeconds :type Float%20%28single-precision%29)))

(fn ConstructionScript)