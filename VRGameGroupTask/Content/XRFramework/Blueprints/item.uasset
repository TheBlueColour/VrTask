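; Grabbable XR pickup item that plays a collection effect and removes itself when grabbed.
; Its Niagara effect starts deactivated on BeginPlay.
; On the grab component's OnGrabbed, it plays a metallic shimmer sound, then after a delay hides a component and activates the Niagara effect.
; After a second delay it destroys the actor.
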(event OnGrabbed(BP_GrabComponent)
  (Audio|PlaySound2D "/Game/Music/SFX_ANIME_Metallic_Shimmer_001.SFX_ANIME_Metallic_Shimmer_001" 1.0 1.0 0.0 0 0)
  (Utilities|FlowControl|Delay 1.0)
  (Rendering|SetVisibility (Variables|Default|Get#) false false)
  (Components|Activation|Activate (Variables|Default|GetNiagara) true)
  (Utilities|FlowControl|Delay 1.0)
  (Actor|DestroyActor))

(event EventBeginPlay
  (Components|Activation|Deactivate (Variables|Default|GetNiagara)))

(fn ConstructionScript)